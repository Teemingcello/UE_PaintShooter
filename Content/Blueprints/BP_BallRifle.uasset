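; BP_BallRifle is a paintball rifle pickup that attaches to the overlapping rifle character's hand socket and binds to its fire and refill events.
; Single shots and timer-driven automatic fire drain ammo by different amounts, with automatic fire stopping when empty.
; Projectiles spawn through a Server-to-Multicast event relay.
; A recursive delayed event refills ammo while not shooting, and separate events show or remove the ammo widget.
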(event OnComponentBeginOverlap(SphereCollision)
  (params (OverlappedComponent :type Primitive%20Component%20Object%20Reference) (OtherActor :type Actor%20Object%20Reference) (OtherComp :type Primitive%20Component%20Object%20Reference) (OtherBodyIndex :type Integer) (bFromSweep :type Boolean) (SweepResult :type Hit%20Result%20Structure%20%28by%20ref%29))
  (bind _asbp_rifle_character (Utilities|Casting|CastToBP_RifleCharacter OtherActor)
    (:then
      (Variables|Default|SetCharacterReference _asbp_rifle_character)
      (Transformation|AttachComponentToComponent self (Variables|/Script/Engine.Character|GetMesh (Variables|Default|GetCharacterReference)) "Weapon_r_Socket" "SnapToTarget" "SnapToTarget" "SnapToTarget" true)
      (Collision|SetCollisionEnabled (Variables|Default|GetSphereCollision) "NoCollision")
      (CallFunction|BallRefill)
      (EventDispatchers|AssignOnFireGun (Variables|Default|GetCharacterReference) (EventDispatchers|CreateEvent :!event Custom|OnFireGun))
      (EventDispatchers|BindEventtoOnFireAutomaticGun (Variables|Default|GetCharacterReference) (EventDispatchers|CreateEvent :!event Custom|OnFireAutomaticGun))
      (EventDispatchers|BindEventtoOnStopAutomaticGun (Variables|Default|GetCharacterReference) (EventDispatchers|CreateEvent :!event Custom|OnStopAutomaticGun))
      (EventDispatchers|BindEventtoOnRefillAmmo (Variables|Default|GetCharacterReference) (EventDispatchers|CreateEvent :!event Custom|BallRefill)))
    (:CastFailed
      (Development|PrintString "Cast to BP_FirstPersonCharacter FAILED"))))

(event Custom|OnFireAutomaticGun
  ;[1 1 1] 자동 연사
  (Variables|Default|SetIsShooting? true)
  (if (not (Variables|Rendering|GetbHidden))
    (Utilities|Time|SetTimerbyFunctionName 0 "OnAutoFireProjectile" (Variables|Weapon|GetAutomaticFireInterval) true)))

(event Custom|OnFireProjectile
  ;[1 1 1] 일반발사 과정
  (CallFunction|ServeronSpawn "/Game/Projectile/BallPaint/BP_BallPaintProjectile.BP_BallPaintProjectile_C" (Transformation|GetWorldTransform (Variables|Default|GetArrow)) "Undefined")
  (CallFunction|BallDrain)
  (Audio|PlaySound2D "/Game/FPWeapon/Audio/FirstPersonTemplateWeaponFire02.FirstPersonTemplateWeaponFire02" 1.0 1.0 0.0 0 0))

(event Custom|BallDrain
  ;[1 1 1] 볼 탄약 감소
  (if (Variables|Default|GetIsShooting?)
    (if (> (Variables|Default|GetAmmo) 0)
      (Variables|Default|SetAmmo (- (Variables|Default|GetAmmo) 15))
      (if (< (Variables|Default|GetAmmo) 0)
        (Variables|Default|SetAmmo 0)))))

(event Custom|ServerOnSpawn
  (params (Class :type Actor%20Class%20Reference) (SpawnTransform :type Transform) (CollisionHandlingOverride :type ESpawnActorCollisionHandlingMethod%20Enum :default "Undefined") (Owner :type Actor%20Object%20Reference) (Instigator :type Pawn%20Object%20Reference))
  ;[1 1 1] Projectile Spawn
  (CallFunction|MulticastonSpawn Class SpawnTransform CollisionHandlingOverride Owner Instigator))

(event Custom|MulticastOnSpawn
  (params (Class :type Actor%20Class%20Reference) (SpawnTransform :type Transform) (CollisionHandlingOverride :type ESpawnActorCollisionHandlingMethod%20Enum :default "Undefined") (Owner :type Actor%20Object%20Reference) (Instigator :type Pawn%20Object%20Reference))
  ;[1 1 1] Projectile Spawn
  (Game|SpawnActorfromClass Class SpawnTransform CollisionHandlingOverride Owner Instigator))

(event Custom|BallAutoDrain
  ;[1 1 1] 볼 자동연사 탄약 감소
  (if (Variables|Default|GetIsShooting?)
    (if (> (Variables|Default|GetAmmo) 0)
      (Variables|Default|SetAmmo (- (Variables|Default|GetAmmo) 5))
      (if (< (Variables|Default|GetAmmo) 0)
        (Variables|Default|SetAmmo 0)))))

(event Custom|OnStopAutomaticGun
  ;[1 1 1] 자동 연사 중지
  (Variables|Default|SetIsShooting? false)
  (Utilities|Time|ClearTimerbyFunctionName 0 "OnAutoFireProjectile"))

(event Custom|BallRefill
  ;[1 1 1] 탄약 리필
  (if (and (< (Variables|Default|GetAmmo) (Variables|Default|GetMaxAmmo)) (== (Variables|Default|GetIsShooting?) false))
    (Utilities|FlowControl|Delay 0.05)
    (bind _output_get (Variables|Default|SetAmmo (+ (Variables|Default|GetAmmo) 1)))
    (if (> _output_get (Variables|Default|GetMaxAmmo))
      (Variables|Default|SetAmmo (Variables|Default|GetMaxAmmo)))
    (CallFunction|BallRefill)))

(event Custom|OnAutoFireProjectile
  ;[1 1 1] 자동연사 발사과정
  (CallFunction|ServeronSpawn "/Game/Projectile/BallPaint/BP_BallPaintProjectile.BP_BallPaintProjectile_C" (Transformation|GetWorldTransform (Variables|Default|GetArrow)) "Undefined")
  (CallFunction|BallAutoDrain)
  (Audio|PlaySound2D "/Game/FPWeapon/Audio/FirstPersonTemplateWeaponFire02.FirstPersonTemplateWeaponFire02" 1.0 1.0 0.0 0 0)
  (if (< (Variables|Default|GetAmmo) 1)
    (Utilities|Time|ClearTimerbyFunctionName 0 "OnAutoFireProjectile")
    (Variables|/Game/Blueprints/BP_RifleCharacter.BP_RifleCharacter_C|SetAuto%20Fire (Variables|Default|GetCharacterReference) false)))

(event Custom|OnFireGun
  ;[1 1 1] 일반 발사
  (Variables|Default|SetIsShooting? true)
  (if (not (Variables|Rendering|GetbHidden))
    (if (< (Variables|Default|GetAmmo) 15)
      (Utilities|FlowControl|Delay 1.0)
      (else
        (CallFunction|OnFireProjectile)))))

(event EventCreateWidget
  ;[1 1 1] 위젯 노출
  (bind _returnvalue (UserInterface|CreateWidget "/Game/UI/WD_BallAmmoCount.WD_BallAmmoCount_C"))
  (bind _output_get (Variables|Default|SetCurrentWidget _returnvalue))
  (UserInterface|Viewport|AddtoViewport _output_get 0)
  (Class|BPIWidgetSetNewWeapon|SetNewWeapon(Message) (Variables|Default|GetCurrentWidget) self))

(event EventRemoveWidget
  ;[1 1 1] 위젯 노출
  (Utilities|IsValid (Variables|Default|GetCurrentWidget)
    (:Is%20Valid
      (Widget|RemovefromParent (Variables|Default|GetCurrentWidget)))))

(fn ConstructionScript)

(fn OnRepColor)

(fn GetWeaponSocket
  (params (Socket%20Name :type Name :default "None"))
  (return ""))